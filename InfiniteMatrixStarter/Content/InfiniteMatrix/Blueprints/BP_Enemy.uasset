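; BP_Enemy is an enemy actor that damages the player on contact and awards score when hit by a bullet.
; Any hit destroys its hit component, then either damages the player or deletes the bullet and increments player score.
; The actor destroys itself only if the damaged player survives; otherwise it flags death and shows restart.
; A Shoot function, not called here, spawns short-lived BP_Bullets from ProjectileSpawnLocation.
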(event `self.ReceiveBeginPlay`)

(event `self.Enemy.OnComponentHit`
  (params (HitComponent :type "PrimitiveComponent Object Reference") (OtherActor :type "Actor Object Reference") (OtherComp :type "PrimitiveComponent Object Reference") (NormalImpulse :type "Vector Structure") (Hit :type "HitResult Structure (by ref)"))
  (`ActorComponent.K2_DestroyComponent` HitComponent)
  (bind _asbp_player (cast `/Game/InfiniteMatrix/Blueprints/BP_Player` OtherActor)
    (:`then`
      (`GameplayStatics.ApplyDamage` _asbp_player 25.0)
      (if (<= (`/Game/InfiniteMatrix/Blueprints/BP_Player.Health` _asbp_player) 0.0)
        (set `/Game/InfiniteMatrix/Blueprints/BP_Player.IsDead` true _asbp_player)
        (`/Game/InfiniteMatrix/Blueprints/BP_Player.DisplayRestart` _asbp_player)
        (else
          (`self.K2_DestroyActor`))))
    (:`CastFailed`
      (bind _asbp_bullet (cast `/Game/InfiniteMatrix/Blueprints/BP_Bullet` OtherActor))
      (`/Game/InfiniteMatrix/Blueprints/BP_Bullet.DeleteBullet` _asbp_bullet)
      (bind _asbp_player_2 (cast `/Game/InfiniteMatrix/Blueprints/BP_Player` (`GameplayStatics.GetPlayerPawn` 0)))
      (set `/Game/InfiniteMatrix/Blueprints/BP_Player.Score` (+ (`/Game/InfiniteMatrix/Blueprints/BP_Player.Score` _asbp_player_2) 1) _asbp_player_2))))

(fn `Shoot`
  (bind _returnvalue (`|SpawnActorFromClass` "/Game/InfiniteMatrix/Blueprints/BP_Bullet.BP_Bullet_C" (`SceneComponent.K2_GetComponentToWorld` (`self.ProjectileSpawnLocation`)) "AlwaysSpawn" "MultiplyWithRoot" null null))
  (`self.SetLifeSpan` _returnvalue 2.0))

(fn `UserConstructionScript`)