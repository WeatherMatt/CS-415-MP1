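; BP_Tunnel is one segment of an endless tunnel, with a spinning holed wall, score trigger and either a health pack or an enemy.
; Randomize functions pick the wall's mesh, rotation, speed and material, and place the pickup or attach a BP_Enemy.
; Hitting the wall damages the player and blocks that segment's point; health packs heal, and both absorb bullets.
; The end trigger asks TunnelSpawner for another segment, then destroys this one and its enemy.
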(event `self.HealthPack.OnComponentHit`
  (params (HitComponent :type "PrimitiveComponent Object Reference") (OtherActor :type "Actor Object Reference") (OtherComp :type "PrimitiveComponent Object Reference") (NormalImpulse :type "Vector Structure") (Hit :type "HitResult Structure (by ref)"))
  (`ActorComponent.K2_DestroyComponent` HitComponent)
  (bind _asbp_player (cast `/Game/InfiniteMatrix/Blueprints/BP_Player` OtherActor)
    (:`then`
      (set `/Game/InfiniteMatrix/Blueprints/BP_Player.Health` (`KismetMathLibrary.FClamp` (+ (`/Game/InfiniteMatrix/Blueprints/BP_Player.Health` _asbp_player) 25.0) 0.0 (`/Game/InfiniteMatrix/Blueprints/BP_Player.MaxHealth` _asbp_player)) _asbp_player))
    (:`CastFailed`
      (bind _asbp_bullet (cast `/Game/InfiniteMatrix/Blueprints/BP_Bullet` OtherActor))
      (`/Game/InfiniteMatrix/Blueprints/BP_Bullet.DeleteBullet` _asbp_bullet))))

(event `self.ReceiveTick`
  (params (DeltaSeconds :type "Float (single-precision)"))
  (`SceneComponent.K2_AddLocalRotation` (`self.WallMesh`) (`KismetMathLibrary.MakeRotator` (* DeltaSeconds (`self.RotateSpeed`))) false false))

(event `self.TriggerZone.OnComponentBeginOverlap`
  (params (OverlappedComponent :type "PrimitiveComponent Object Reference") (OtherActor :type "Actor Object Reference") (OtherComp :type "PrimitiveComponent Object Reference") (OtherBodyIndex :type Integer) (bFromSweep :type Boolean) (SweepResult :type "HitResult Structure (by ref)"))
  (bind _enemy (`self.Enemy`))
  (cast `/Game/InfiniteMatrix/Blueprints/BP_Player` OtherActor)
  (`/Game/InfiniteMatrix/Blueprints/BP_TunnelSpawner.SpawnTunnelAtSpawnPoint` (`self.TunnelSpawner`))
  (`self.K2_DestroyActor`)
  (`/Engine/EditorBlueprintResources/StandardMacros.IsValid` _enemy
    (:`Is Valid`
      (`self.K2_DestroyActor` _enemy))))

(event `self.WallMesh.OnComponentHit`
  (params (HitComponent :type "PrimitiveComponent Object Reference") (OtherActor :type "Actor Object Reference") (OtherComp :type "PrimitiveComponent Object Reference") (NormalImpulse :type "Vector Structure") (Hit :type "HitResult Structure (by ref)"))
  (bind _asbp_player (cast `/Game/InfiniteMatrix/Blueprints/BP_Player` OtherActor)
    (:`then`
      (`GameplayStatics.ApplyDamage` _asbp_player 25.0)
      (if (<= (`/Game/InfiniteMatrix/Blueprints/BP_Player.Health` _asbp_player) 0.0)
        (set `/Game/InfiniteMatrix/Blueprints/BP_Player.IsDead` true _asbp_player)
        (`/Game/InfiniteMatrix/Blueprints/BP_Player.DisplayRestart` _asbp_player)
        (else
          (`PrimitiveComponent.SetCollisionEnabled` (`self.WallMesh`) "NoCollision")
          (set `self.HitWall` true))))
    (:`CastFailed`
      (bind _asbp_bullet (cast `/Game/InfiniteMatrix/Blueprints/BP_Bullet` OtherActor))
      (`/Engine/EditorBlueprintResources/StandardMacros.IsValid` _asbp_bullet
        (:`Is Valid`
          (`self.K2_DestroyActor` _asbp_bullet))))))

(event `self.ScoreTrigger.OnComponentBeginOverlap`
  (params (OverlappedComponent :type "PrimitiveComponent Object Reference") (OtherActor :type "Actor Object Reference") (OtherComp :type "PrimitiveComponent Object Reference") (OtherBodyIndex :type Integer) (bFromSweep :type Boolean) (SweepResult :type "HitResult Structure (by ref)"))
  (bind _asbp_player (cast `/Game/InfiniteMatrix/Blueprints/BP_Player` OtherActor))
  (if (not (`self.HitWall`))
    (set `/Game/InfiniteMatrix/Blueprints/BP_Player.Score` (+ (`/Game/InfiniteMatrix/Blueprints/BP_Player.Score` _asbp_player) 1) _asbp_player)))

(fn `RandomizeHealthPack`
  (if (== (`KismetMathLibrary.RandomIntegerInRange` 0 4) 0)
    (`SceneComponent.K2_SetRelativeLocation` (`self.HealthPack`) (`KismetMathLibrary.MakeVector` (`KismetMathLibrary.RandomFloatInRange` 500.0 2000.0) (`KismetMathLibrary.RandomFloatInRange` -200.0 200.0) (`KismetMathLibrary.RandomFloatInRange` -200.0 200.0)) false true)
    (else
      (`ActorComponent.K2_DestroyComponent` (`self.HealthPack`))
      (if (== (`KismetMathLibrary.RandomIntegerInRange` 0) 0)
        (bind _returnvalue (`|SpawnActorFromClass` "/Game/InfiniteMatrix/Blueprints/BP_Enemy.BP_Enemy_C" (`KismetMathLibrary.MakeTransform` (0.0 0.0 0.0)) "Undefined" "MultiplyWithRoot" null null))
        (`self.K2_AttachToComponent` _returnvalue (`self.StaticMeshComponent`) "None" "KeepRelative" "KeepRelative" "KeepRelative" true)
        (`self.K2_SetActorRelativeLocation` _returnvalue (`KismetMathLibrary.MakeVector` (`KismetMathLibrary.RandomFloatInRange` 500.0 2000.0) (`KismetMathLibrary.RandomFloatInRange` -200.0 200.0) (`KismetMathLibrary.RandomFloatInRange` -200.0 200.0)) false false)
        (set `self.Enemy` _returnvalue)))))

(fn `RandomizeWall`
  (bind _returnvalue (`KismetMathLibrary.RandomFloatInRange` 50.0 160.0))
  (`StaticMeshComponent.SetStaticMesh` (`self.WallMesh`) (select `int` (`KismetMathLibrary.RandomIntegerInRange` 0 3) :`0` "/Game/InfiniteMatrix/Meshes/SM_Hole_01.SM_Hole_01" :`1` "/Game/InfiniteMatrix/Meshes/SM_Hole_02.SM_Hole_02" :`2` "/Game/InfiniteMatrix/Meshes/SM_Hole_03.SM_Hole_03" :`3` "/Game/InfiniteMatrix/Meshes/SM_Hole_04.SM_Hole_04" :!type "StaticMesh Object Reference"))
  (`SceneComponent.K2_AddLocalRotation` (`self.WallMesh`) (`KismetMathLibrary.MakeRotator` (`KismetMathLibrary.RandomFloatInRange` 0.0 360.0)) false false)
  (set `self.RotateSpeed` _returnvalue)
  (if (> _returnvalue 120.0)
    (`PrimitiveComponent.SetMaterial` (`self.WallMesh`) 0 "/Engine/EngineDebugMaterials/BoneWeightMaterial.BoneWeightMaterial")))

(fn `UserConstructionScript`)