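; BP_TunnelSpawner builds a chain of BP_Tunnel segments, starting at the player pawn's location.
; On BeginPlay it destroys existing tunnels and their enemies, then spawns a short initial run of segments.
; Each segment attaches at the SpawnPoint of the newest one, which the spawner tracks.
; New tunnels receive a reference to the spawner and randomize their wall and health pack.
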(event `self.ReceiveBeginPlay`
  (`self.SpawnInitialTunnels`))

(fn `SpawnInitialTunnels`
  (`|ExecutionSequence`
    (:`then_0`
      (bind _outactors (`GameplayStatics.GetAllActorsOfClass` "/Game/InfiniteMatrix/Blueprints/BP_Tunnel.BP_Tunnel_C"))
      (for _array_element _outactors
        (bind _asbp_tunnel (cast `/Game/InfiniteMatrix/Blueprints/BP_Tunnel` _array_element))
        (bind _enemy (`/Game/InfiniteMatrix/Blueprints/BP_Tunnel.Enemy` _asbp_tunnel))
        (`/Engine/EditorBlueprintResources/StandardMacros.IsValid` _enemy
          (:`Is Valid`
            (`self.K2_DestroyActor` _enemy))
          (:`Is Not Valid`
            _))
        (`self.K2_DestroyActor` _array_element)))
    (:`then_1`
      (for _ (range 3)
        (`/Engine/EditorBlueprintResources/StandardMacros.IsValid` (`self.NewestTunnel`)
          (:`Is Valid`
            (`self.SpawnTunnelAtSpawnPoint`))
          (:`Is Not Valid`
            (`self.SpawnTunnel` (`self.K2_GetActorLocation` (`GameplayStatics.GetPlayerPawn` 0)))))))))

(fn `SpawnTunnel`
  (params (SpawnLoaction :type "Vector Structure"))
  (bind _returnvalue (`|SpawnActorFromClass` "/Game/InfiniteMatrix/Blueprints/BP_Tunnel.BP_Tunnel_C" (`KismetMathLibrary.MakeTransform` SpawnLoaction) "Undefined" "MultiplyWithRoot" null null))
  (bind _output_get (set `self.NewestTunnel` _returnvalue))
  (set `/Game/InfiniteMatrix/Blueprints/BP_Tunnel.TunnelSpawner` self _output_get)
  (`/Game/InfiniteMatrix/Blueprints/BP_Tunnel.RandomizeWall` _output_get)
  (`/Game/InfiniteMatrix/Blueprints/BP_Tunnel.RandomizeHealthPack` (`self.NewestTunnel`)))

(fn `SpawnTunnelAtSpawnPoint`
  (`self.SpawnTunnel` (`SceneComponent.K2_GetComponentLocation` (`/Game/InfiniteMatrix/Blueprints/BP_Tunnel.SpawnPoint` (`self.NewestTunnel`)))))

(fn `UserConstructionScript`
  (`parent.UserConstructionScript`))